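; Spline-driven placement actor, named as a concrete fence, that builds a deformed mesh along an editable spline.
; The construction script adds one SplineMeshComponent per segment between consecutive spline points, using their local positions and tangents to bend it.
; The Width variable sets both start and end cross-section scale for every segment.
; It has no runtime logic, and a forward-axis setter node is left disconnected.
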(event EventBeginPlay)

(event Collision|EventActorBeginOverlap
  (params (OtherActor :type Actor%20Object%20Reference)))

(event EventTick
  (params (DeltaSeconds :type Float%20%28single-precision%29)))

(fn ConstructionScript
  (bind _spline (Variables|Default|GetSpline))
  (bind _spline_2 (Variables|Default|GetSpline))
  (bind _width (Variables|Default|GetWidth))
  (bind _returnvalue (Math|Conversions|ToVector2D(Vector) _width))
  (for _index (range 0 (- (Spline|GetNumberOfSplinePoints (Variables|Default|GetSpline)) 2))
    (bind _returnvalue_2 (AddComponent|AddSplineMeshComponent false))
    (SplineMesh|SetStartScale _returnvalue_2 _returnvalue true :!class /Script/Engine.SplineMeshComponent)
    (SplineMesh|SetEndScale _returnvalue_2 _returnvalue true :!class /Script/Engine.SplineMeshComponent)
    (SplineMesh|SetStartandEnd _returnvalue_2 (Spline|GetLocationatSplinePoint _spline_2 _index "Local") (Spline|GetTangentatSplinePoint _spline_2 _index "Local") (Spline|GetLocationatSplinePoint _spline (+ _index 1) "Local") (Spline|GetTangentatSplinePoint _spline (+ _index 1) "Local") true :!class /Script/Engine.SplineMeshComponent)))